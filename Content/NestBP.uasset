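; Wildlife nest actor that spawns creatures around itself and glows in the color of its maximum rarity.
; On BeginPlay with authority, it rotates a pivot in even steps and spawns one WildLife per rarity tier up to MaxRarity, passing itself as HomeNest.
; GetRarityColor maps the five tiers, Common to Legendary, to the point light color, applied in the construction script and again while spawning.
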(event EventBeginPlay
  (bind _max_rarity (Variables|Default|GetMax%20Rarity))
  (bind _returnvalue (Math|Byte|MakeLiteralByte _max_rarity))
  (bind _returnvalue_2 (Math|Conversions|ToInteger(Byte) _returnvalue))
  (Networking|SwitchHasAuthority
    (:Authority
      (for _index (range 0 _returnvalue_2)
        (Transformation|SetRelativeRotation (Variables|Default|GetWildLife%20Spawn%20Pivot) (Math|Rotator|MakeRotator 0.0 0.0 (* _index (/ 3.6e+02 (Math|Conversions|ToFloat(Integer) (+ _returnvalue_2 1))))) false false)
        (Game|SpawnActorfromClass "/Game/WildLife.WildLife_C" (Transformation|GetWorldTransform (Variables|Default|GetWildLife%20Spawn)) "Undefined" 0 self 0)
        (Rendering|Components|Light|SetLightColor (Variables|Default|GetPointLight) (CallFunction|GetRarityColor (Variables|Default|GetMax%20Rarity)) true)))))

(fn ConstructionScript
  (Rendering|Components|Light|SetLightColor (Variables|Default|GetPointLight) (CallFunction|GetRarityColor (Variables|Default|GetMax%20Rarity)) true))

(fn GetRarityColor
  (params (Rarity :type Rarity%20Enum :default "NewEnumerator0"))
  (switch Utilities|FlowControl|Switch|SwitchonRarity Rarity
    (:NewEnumerator0
      (return "(R=0.765625,G=0.765625,B=0.765625,A=1.000000)"))
    (:NewEnumerator1
      (return "(R=0.119792,G=1.000000,B=0.119792,A=1.000000)"))
    (:NewEnumerator2
      (return "(R=0.079322,G=0.078125,B=1.000000,A=1.000000)"))
    (:NewEnumerator3
      (return "(R=0.986009,G=0.041667,B=1.000000,A=1.000000)"))
    (:NewEnumerator4
      (return "(R=0.968750,G=0.508664,B=0.000000,A=1.000000)"))))